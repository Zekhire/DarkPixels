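; Enemy Blueprint that tracks the nearest Avatar_BP and takes damage until it is marked dead.
; While FollowPlayers is set, Tick rescans all avatars for the closest, but the AIMoveTo toward it is unconnected.
; ApplyDamage lowers Health; on death it searches BP_EventHandler's OutActors for the name stored by PlayerName and increases that actor's initial damage by DamageMultiplayer.
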(event Custom|GetTheClosestPlayer
  (bind _self self)
  (bind _returnvalue (Transformation|GetActorLocation _self))
  (bind _outactors (Actor|GetAllActorsOfClass "/Game/Avatar_BP.Avatar_BP_C"))
  (bind _output_get (Variables|Default|SetPlayers _outactors))
  (Variables|Default|SetTheClosestPlayer (Utilities|Array|Get(acopy) _output_get))
  (for _index (range 1 (- (Utilities|Array|Length _output_get) 1))
    (if (not (< (Math|Vector|Distance(Vector) _returnvalue (Transformation|GetActorLocation (Variables|Default|GetTheClosestPlayer))) (Math|Vector|Distance(Vector) (Transformation|GetActorLocation (Utilities|Array|Get(acopy) (Variables|Default|GetPlayers) _index)) _returnvalue)))
      (Variables|Default|SetTheClosestPlayer (Utilities|Array|Get(acopy) (Variables|Default|GetPlayers) _index)))))

(event EventBeginPlay
  (bind _returnvalue (Actor|GetActorOfClass "/Game/Custom/BP_EventHandler.BP_EventHandler_C"))
  (Variables|Default|SetEventHandler _returnvalue))

(event Collision|EventActorBeginOverlap
  (params (OtherActor :type Actor%20Object%20Reference)))

(event EventTick
  (params (DeltaSeconds :type Float%20%28single-precision%29))
  (if (Variables|Default|GetFollowPlayers)
    (CallFunction|GettheClosestPlayer)))

(event EventApplyDamage
  (params (DamageAmount :type Float%20%28double-precision%29))
  (if (Variables|Default|GetisAlive?)
    (Variables|Default|SetHealth (- (Variables|Default|GetHealth) DamageAmount))
    (if (<= (Variables|Default|GetHealth) 0.0)
      (Variables|Default|SetisAlive? false)
      (bind _array_element (Utilities|Array|ForEachLoopwithBreak (Variables|/Game/Custom/BP_EventHandler.BP_EventHandler_C|GetOut%20Actors (Variables|Default|GetEventHandler)))
        (:LoopBody
          (if (Utilities|Enum|Equal(Enum) (Variables|/Game/Avatar_BP.Avatar_BP_C|GetActorName _array_element) (Variables|Default|GetActive%20Player))
            (Default|IncreaseInitialDamage _array_element (Variables|Default|GetDamageMultiplayer)))))
      (else
        (Development|PrintString (Utilities|String|ToString(Float) (Variables|Default|GetHealth)))))))

(event EventPlayerName
  (params (ActivePlayer :type String))
  (bind _output_get (Variables|Default|SetActive%20Player ActivePlayer))
  (Development|PrintString (Utilities|String|Append "Enemy --> " _output_get)))

(fn ConstructionScript)