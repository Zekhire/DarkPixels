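; BP_Target is a damageable target actor that stores the active player's name and is meant to show damage on a widget HUD.
; Its logic subtracts damage from Health, reports it per player, and on death notifies BP_EventHandler to increase that player's damage, then resets Health.
; The damage and HUD setup chains are disconnected from ApplyDamage and BeginPlay, so as wired only PlayerName does anything.
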(event EventBeginPlay)

(event Collision|EventActorBeginOverlap
  (params (OtherActor :type Actor%20Object%20Reference)))

(event EventTick
  (params (DeltaSeconds :type Float%20%28single-precision%29)))

(event EventApplyDamage
  (params (DamageAmount :type Float%20%28double-precision%29)))

(event EventPlayerName
  (params (ActivePlayer :type String))
  (Variables|Default|SetActive%20Player ActivePlayer))

(fn ConstructionScript)