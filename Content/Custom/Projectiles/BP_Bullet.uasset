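; Bullet projectile that delivers damage, its owning player and a push vector to whatever it hits.
; ApplyDamage and PlayerName events store the damage amount and active player, with the damage also printed on screen.
; When the Sphere overlaps an actor implementing BPI_Global, it passes both values plus a scaled, Z-flattened forward vector through interface messages, then destroys itself.
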(event OnComponentBeginOverlap(Sphere)
  (params (OverlappedComponent :type Primitive%20Component%20Object%20Reference) (OtherActor :type Actor%20Object%20Reference) (OtherComp :type Primitive%20Component%20Object%20Reference) (OtherBodyIndex :type Integer) (bFromSweep :type Boolean) (SweepResult :type Hit%20Result%20Structure%20%28by%20ref%29))
  (bind _sphere (Variables|Default|GetSphere))
  (bind _returnvalue (Transformation|GetWorldRotation _sphere))
  (bind _returnvalue_2 (Math|Vector|GetForwardVector _returnvalue))
  (if (Utilities|DoesObjectImplementInterface OtherActor "/Game/Custom/Projectiles/BPI_Global.BPI_Global_C")
    (Utilities|IsValid self
      (:Is%20Valid
        (Class|BPIGlobal|PlayerName(Message) OtherActor (Variables|Default|GetActivePlayer))
        (Class|BPIGlobal|ApplyDamage(Message) OtherActor (Variables|Default|GetDamage%20Amount))
        (Class|BPIGlobal|DamageVector(Message) OtherActor (* (Math|Vector|MakeVector (.x _returnvalue_2) (.y _returnvalue_2) 0.0) 1e+04))
        (Actor|DestroyActor)))))

(event EventBeginPlay)

(event Collision|EventActorBeginOverlap
  (params (OtherActor :type Actor%20Object%20Reference)))

(event EventTick
  (params (DeltaSeconds :type Float%20%28single-precision%29)))

(event EventPlayerName
  (params (ActivePlayer :type String))
  (Variables|Default|SetActivePlayer ActivePlayer))

(event EventApplyDamage
  (params (DamageAmount :type Float%20%28double-precision%29))
  (bind _output_get (Variables|Default|SetDamage%20Amount DamageAmount))
  (Development|PrintString (Utilities|String|ToString(Float) _output_get) true true "(R=1.000000,G=0.250000,B=0.000000,A=1.000000)"))

(fn ConstructionScript)