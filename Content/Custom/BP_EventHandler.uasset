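; BP_EventHandler is an event relay actor that triggers damage increases on Avatar_BP player actors.
; One second after BeginPlay, it caches all Avatar_BP actors in an array.
; PlayerName stores the active player and prints it for debugging.
; IncreaseDamageforPlayer loops over the cached avatars and, behind a Player equality check that does not reference the loop element, calls IncreaseInitialDamageMessage on each with DamageMultiplayer.
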(event EventBeginPlay
  (Utilities|FlowControl|Delay 1.0)
  (bind _outactors (Actor|GetAllActorsOfClass "/Game/Avatar_BP.Avatar_BP_C"))
  (Variables|Default|SetOut%20Actors _outactors))

(event Collision|EventActorBeginOverlap
  (params (OtherActor :type Actor%20Object%20Reference)))

(event EventTick
  (params (DeltaSeconds :type Float%20%28single-precision%29)))

(event EventIncreaseDamageforPlayer
  (params (Player :type String))
  (for _array_element (Variables|Default|GetOut%20Actors)
    (if (Utilities|Enum|Equal(Enum) Player (Variables|Default|GetPlayer))
      (Class|BPIGlobal|IncreaseInitialDamage(Message) _array_element (Variables|Default|GetDamageMultiplayer)))))

(event EventPlayerName
  (params (ActivePlayer :type String))
  (bind _output_get (Variables|Default|SetPlayer ActivePlayer))
  (Development|PrintString (Utilities|String|Append "EventHandler --> " _output_get) true true "(R=1.000000,G=0.250000,B=0.000000,A=1.000000)"))

(fn ConstructionScript)