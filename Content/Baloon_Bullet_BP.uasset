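; Balloon bullet actor that lifts an enemy into the air, hanging it by the neck as a ragdoll.
; FlyEnemyAway spawns and attaches a cable and a physics constraint, linking both to the enemy's Neck.
; It also stops the enemy following players, disables its movement, clears its animation, enables mesh physics and plays a sound.
; Once FlyUp is set, Tick raises the balloon a fixed step every frame.
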(event Custom|FlyEnemyAway
  (params (Enemy :type Enemy%20BP%20Object%20Reference))
  (bind _self self)
  (bind _mesh (Variables|/Script/Engine.Character|GetMesh Enemy))
  (bind _returnvalue (Transformation|GetActorLocation _self))
  (Variables|Default|SetFlyUp true)
  (bind _returnvalue_2 (Game|SpawnActorfromClass "/Script/Engine.PhysicsConstraintActor" (Math|Transform|MakeTransform (Math|Vector|MakeVector (.x _returnvalue) (.y _returnvalue) (- (.z _returnvalue) 1e+02)) "0, 0, 0" "1.000000,1.000000,1.000000") "Undefined" "MultiplyWithRoot" 0 0))
  (Transformation|AttachActorToActor _returnvalue_2 self "None" "KeepWorld" "KeepWorld" "KeepWorld" true)
  (bind _returnvalue_3 (Game|SpawnActorfromClass "/Script/CableComponent.CableActor" (Math|Transform|MakeTransform (Transformation|GetActorLocation self) "0, 0, 0" "1.000000,1.000000,1.000000") "Undefined" "MultiplyWithRoot" 0 0))
  (Transformation|AttachActorToActor _returnvalue_3 self "None" "KeepWorld" "KeepWorld" "KeepWorld" true)
  (Class|CableComponent|SetAttachEndto (Variables|/Script/CableComponent.CableActor|GetCableComponent _returnvalue_3) Enemy "Mesh" "Neck")
  (Variables|/Script/CableComponent.CableComponent|SetEndLocation (Variables|/Script/CableComponent.CableActor|GetCableComponent _returnvalue_3) "0, 0, 0")
  (Class|PhysicsConstraintComponent|SetConstrainedComponents (Variables|/Script/Engine.PhysicsConstraintActor|GetConstraintComp _returnvalue_2) (Variables|Default|GetSphere) "None" (Variables|/Script/Engine.Character|GetMesh Enemy) "Neck")
  (Variables|/Game/Enemy_BP.Enemy_BP_C|SetFollowPlayers Enemy false)
  (Class|SkeletalMeshComponent|SetAnimClass _mesh)
  (Pawn|Components|CharacterMovement|SetMovementMode (Variables|/Script/Engine.Character|GetCharacterMovement Enemy) "MOVE_None" 0)
  (Physics|SetSimulatePhysics _mesh true)
  (Collision|SetCollisionProfileName _mesh "BlockAll" true :!class /Script/Engine.PrimitiveComponent)
  (Variables|Default|SetFlyUp true)
  (Audio|PlaySound2D 0 1.0 1.0 0.0 0 0))

(event Custom|FlyStart)

(event EventBeginPlay)

(event Collision|EventActorBeginOverlap
  (params (OtherActor :type Actor%20Object%20Reference)))

(event EventTick
  (params (DeltaSeconds :type Float%20%28single-precision%29))
  (bind _self self)
  (bind _returnvalue (Transformation|GetActorLocation _self))
  (if (Variables|Default|GetFlyUp)
    (Transformation|SetActorLocation (Math|Vector|MakeVector (.x _returnvalue) (.y _returnvalue) (+ (.z _returnvalue) 2.0)) false false)))

(fn ConstructionScript)