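; Flying camera actor that becomes the first player's view target at BeginPlay and follows the group of Avatar_BP actors.
; Each Tick it gathers every Avatar_BP with GetAllActorsOfClass and averages their locations into a center point.
; It then moves the Camera to that center minus CameraCenterOffset in X and Y, sweeping the move and keeping its current height.
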(event Custom|ComputeCameraPosition
  (bind _camera (Variables|Default|GetCamera))
  (bind _players (Variables|Default|GetPlayers))
  (Variables|Default|SetCameraCenter "0, 0, 0")
  (for _array_element _players
    (Variables|Default|SetCameraCenter (+ (Variables|Default|GetCameraCenter) (Transformation|GetActorLocation _array_element))))
  (bind _output_get (Variables|Default|SetCameraCenter (/ (Variables|Default|GetCameraCenter) (Utilities|Array|Length _players))))
  (Transformation|SetWorldLocation _camera (Math|Vector|MakeVector (.x (- _output_get (Variables|Default|GetCameraCenterOffset))) (.y (- _output_get (Variables|Default|GetCameraCenterOffset))) (.z (Transformation|GetWorldLocation _camera))) true false))

(event EventBeginPlay
  (Game|Player|SetViewTargetwithBlend (Game|GetPlayerController 0) self 0.0 "VTBlend_Linear" 0.0 false))

(event EventTick
  (params (DeltaSeconds :type Float%20%28single-precision%29))
  (bind _outactors (Actor|GetAllActorsOfClass "/Game/Avatar_BP.Avatar_BP_C"))
  (Variables|Default|SetPlayers _outactors)
  (CallFunction|ComputeCameraPosition))

(event Collision|EventActorBeginOverlap
  (params (OtherActor :type Actor%20Object%20Reference)))

(fn ConstructionScript)