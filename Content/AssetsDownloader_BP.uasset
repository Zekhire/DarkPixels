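; Level actor that kicks off the download of every Spiegel in the game instance's playlists when play begins.
; After a short delay it constructs DarkPixelsSpiegelActions to add its functions to the SpiegelManager.
; It then passes each JSON playlist entry's ID, name and S3 URL, plus the level's SpiegelManager and AssetLibrary, to EmpManager's async download.
; A non-async version of the download call is left unconnected.
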(event EventBeginPlay
  (Utilities|FlowControl|Delay 0.2)
  (bind _returnvalue (Game|ConstructObjectfromClass "/Script/DarkPixels.DarkPixelsSpiegelActions"))
  (Class|ExternalSpiegelFunctionsSet|AddFunctionstoSpiegelManager _returnvalue)
  (bind _asgi_dark_pixels (Utilities|Casting|CastToGI_DarkPixels (Game|GetGameInstance)))
  (for _array_element (Variables|/Game/Data/GI_DarkPixels.GI_DarkPixels_C|GetSpiegelPlaylist _asgi_dark_pixels)
    (bind _returnvalue_2 (Actor|GetActorOfClass "/Script/SpiegelController.SpiegelManager"))
    (bind _returnvalue_3 (Actor|GetActorOfClass "/Script/SpiegelController.AssetLibrary"))
    (Class|EmpManager|DownloadAllSpiegelsBasedonPlaylistIdAsync (Variables|/Game/Data/GI_DarkPixels.GI_DarkPixels_C|GetEmpManager _asgi_dark_pixels) (Class|VaRestJsonObject|GetStringField _array_element "object_id") (Class|VaRestJsonObject|GetStringField _array_element "object_name") (Class|VaRestJsonObject|GetStringField _array_element "s3_playlist_url") _returnvalue_2 _returnvalue_3 false)))

(event Collision|EventActorBeginOverlap
  (params (OtherActor :type Actor%20Object%20Reference)))

(event EventTick
  (params (DeltaSeconds :type Float%20%28single-precision%29)))

(fn ConstructionScript)