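; PadDetector_BP sets up local multiplayer at BeginPlay by creating one player per connected input device beyond the first.
; It adds the main widget, then after a short delay loops over the input devices, using each loop index as controller ID.
; New players' Avatar_BP pawns get an index, skin, name, possession and Enhanced Input mapping, while player 0 only gets its index.
; A separate delayed step displays the players bar.
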(event Custom|SetAvatarSkin
  (params (ControlledPawn :type Pawn%20Object%20Reference) (PlayerIndex :type Integer))
  (bind _asavatar_bp (Utilities|Casting|CastToAvatar_BP ControlledPawn))
  (Components|SkeletalMesh|SetSkeletalMeshAsset (Variables|/Script/Engine.Character|GetMesh _asavatar_bp) (Utilities|Array|Get(acopy) (Variables|Default|GetSkeletals) PlayerIndex))
  (Default|PlayerName _asavatar_bp (Utilities|Array|Get(acopy) (Variables|Default|GetActorNames) PlayerIndex)))

(event EventBeginPlay
  (Utilities|FlowControl|Sequence
    (:then_0
      (bind _returnvalue (UserInterface|CreateWidget "/Game/UMG/Widgets/WDG_MainWidget.WDG_MainWidget_C"))
      (UserInterface|Viewport|AddtoViewport _returnvalue 0)
      (Variables|Default|SetPlayerUIReference (Variables|/Game/UMG/Widgets/WDG_MainWidget.WDG_MainWidget_C|GetWDG_PlayerUI _returnvalue)))
    (:then_1
      (Utilities|FlowControl|Delay 0.2)
      (bind _outinputdevices (Class|InputDeviceLibrary|GetAllConnectedInputDevices))
      (for (_ _array_index) _outinputdevices
        (if (> _array_index 0)
          (bind _returnvalue_2 (Class|GameplayStatics|CreatePlayer _array_index))
          (bind _asavatar_bp (Utilities|Casting|CastToAvatar_BP (Pawn|GetControlledPawn _returnvalue_2)))
          (Default|PlayerIndex _asavatar_bp _array_index)
          (CallFunction|SetAvatarSkin (Pawn|GetControlledPawn _returnvalue_2) _array_index)
          (Pawn|Possess (Game|GetPlayerController _array_index) (Pawn|GetControlledPawn _returnvalue_2))
          (Input|AddMappingContext (PlayerController|LocalPlayerSubsystems|GetEnhancedInputLocalPlayerSubsystem _returnvalue_2) "/Game/NewInputMappingContext.NewInputMappingContext" 0 "(bIgnoreAllPressedKeysUntilRelease=True,bForceImmediately=False)")
          (else
            (bind _asavatar_bp_2 (Utilities|Casting|CastToAvatar_BP (Pawn|GetControlledPawn (Game|GetPlayerController 0))))
            (Default|PlayerIndex _asavatar_bp_2)))))
    (:then_2
      (Utilities|FlowControl|Delay 5.0)
      (Default|DisplayPlayersBar (Variables|Default|GetPlayerUIReference)))))

(event Collision|EventActorBeginOverlap
  (params (OtherActor :type Actor%20Object%20Reference)))

(event EventTick
  (params (DeltaSeconds :type Float%20%28single-precision%29)))

(fn ConstructionScript)